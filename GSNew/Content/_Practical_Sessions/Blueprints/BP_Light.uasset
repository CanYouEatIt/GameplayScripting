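; BP_Light is a practice light actor whose point light animates its brightness and colour during play.
; On BeginPlay a timeline plays, scaling its intensity track by the LightIntensity variable and applying its colour track to the PointLight on each update.
; Unconnected leftover nodes hold earlier experiments with a player-distance on/off switch and a delayed intensity and colour change, and never run.
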(event EventBeginPlay
  (bind (_direction _lightintensity _colour) (Timeline|LightTimeline Play)
    (:Update
      (Rendering|Components|Light|SetIntensity (Variables|Default|GetPointLight) (* _lightintensity (Variables|Default|GetLightIntensity)))
      (Rendering|Components|Light|SetLightColor (Variables|Default|GetPointLight) _colour true))))

(event Collision|EventActorBeginOverlap
  (params (OtherActor :type Actor%20Object%20Reference)))

(event EventTick
  (params (DeltaSeconds :type Float%20%28single-precision%29)))

(fn ConstructionScript)